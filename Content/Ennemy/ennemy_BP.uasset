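; Enemy character that chases the hero once it overlaps the detection box and attacks on reaching it.
; A looping AI MoveTo retries after a short delay, removing one of the hero's lives per successful approach with a pause between hits.
; At zero lives it triggers the hero's GameOver once.
; Its death event sets the animation Blueprint's Dead flag, stops movement and destroys the actor after a delay.
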(event `Attaquer`
  (bind _hero (`self.Hero`))
  ;[1 1 1] Attaquer
  (bind _output_get (set `/Game/Hero/Hero_BP.Vies` (`KismetMathLibrary.Clamp` (- (`/Game/Hero/Hero_BP.Vies` _hero) 1) 0 5) _hero))
  (if (== _output_get 0)
    (`self.Tuer`)
    (else
      (`KismetSystemLibrary.PrintString` "Pas tuer"))))

(event `self.Box.OnComponentBeginOverlap`
  (params (OverlappedComponent :type "PrimitiveComponent Object Reference") (OtherActor :type "Actor Object Reference") (OtherComp :type "PrimitiveComponent Object Reference") (OtherBodyIndex :type Integer) (bFromSweep :type Boolean) (SweepResult :type "HitResult Structure (by ref)"))
  ;[1 1 1] Détéction du héro
  (bind _ashero_bp (cast `/Game/Hero/Hero_BP` OtherActor))
  (set `self.Hero` _ashero_bp)
  (`self.FollowHero`))

(event `FollowHero`
  (bind _hero (`self.Hero`))
  ;[1 1 1] Suivre le héro
  (`|AIMoveTo` _hero self (0.0 0.0 0.0) _hero
    (:`OnSuccess`
      (`self.Attaquer`)
      (`KismetSystemLibrary.Delay` 2.0)
      (`self.FollowHero`))
    (:`OnFail`
      (`KismetSystemLibrary.Delay` 0.2)
      (`self.FollowHero`))))

(event `Tuer`
  ;[1 1 1] Tuer
  (`/Engine/EditorBlueprintResources/StandardMacros.DoOnce` false
    (:`Completed`
      (`/Game/Hero/Hero_BP.GameOver` (`self.Hero`)))))

(event `Mort`
  ;[1 1 1] Mort
  (bind _asennemy_anim_bp (cast `/Game/Ennemy/Animation/Ennemy_Anim_BP` (`SkeletalMeshComponent.GetAnimInstance` (`self.Mesh`))))
  (set `/Game/Ennemy/Animation/Ennemy_Anim_BP.Dead?` true _asennemy_anim_bp)
  (set `CharacterMovementComponent.MaxWalkSpeed` 0.0 (`self.CharacterMovement`))
  (`KismetSystemLibrary.Delay` 1.0)
  (`self.K2_DestroyActor`))

(fn `UserConstructionScript`)