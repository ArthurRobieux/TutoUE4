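; Hero_BP is the player character Blueprint, handling movement, camera look and jumping.
; Axis inputs move the character along the camera's forward and right vectors and feed controller yaw and pitch.
; Pressing Jump starts the jump and sets a Jump flag on the mesh's Lutin_Anim_BP anim instance, which OnLanded clears.
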(event `InputAxis|MoveForward`
  (params (AxisValue :type "Float (single-precision)"))
  ;[1 1 1] Déplacement du personnage
  (`self.AddMovementInput` (`SceneComponent.GetForwardVector` (`self.Camera`)) AxisValue))

(event `InputAxis|MoveRight`
  (params (AxisValue :type "Float (single-precision)"))
  ;[1 1 1] Déplacement du personnage
  (`self.AddMovementInput` (`SceneComponent.GetRightVector` (`self.Camera`)) AxisValue))

(event `InputAxis|Turn`
  (params (AxisValue :type "Float (single-precision)"))
  ;[1 1 1] Orientation de la caméra
  (`self.AddControllerYawInput` AxisValue))

(event `InputAction|Jump`
  (params (Key :type "Key Structure"))
  ;[1 1 1] Saut
  (:`Pressed`
    (`self.Jump`)
    (bind _aslutin_anim_bp (cast `/Game/Hero/Animation/Lutin_Anim_BP` (`SkeletalMeshComponent.GetAnimInstance` (`self.Mesh`))))
    (set `/Game/Hero/Animation/Lutin_Anim_BP.Jump?` true _aslutin_anim_bp)))

(event `InputAxis|LookUp`
  (params (AxisValue :type "Float (single-precision)"))
  ;[1 1 1] Orientation de la caméra
  (`self.AddControllerPitchInput` AxisValue))

(event `self.OnLanded`
  (params (Hit :type "HitResult Structure (by ref)"))
  ;[1 1 1] Atterissage
  (bind _aslutin_anim_bp (cast `/Game/Hero/Animation/Lutin_Anim_BP` (`SkeletalMeshComponent.GetAnimInstance` (`self.Mesh`))))
  (set `/Game/Hero/Animation/Lutin_Anim_BP.Jump?` false _aslutin_anim_bp))

(fn `UserConstructionScript`)