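; Lamp Blueprint whose point light color the player adjusts from the keyboard.
; BeginPlay enables input from player controller 0, so the Multiply and Divide keys raise or lower the red (X) component of the Couleur vector in unit steps, without clamping.
; Tick reapplies Couleur to the PointLight as RGB every frame, with alpha fixed at full.
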(event `self.ReceiveTick`
  (params (DeltaSeconds :type "Float (single-precision)"))
  (bind (_couleur_x _couleur_y _couleur_z) (`KismetMathLibrary.BreakVector` (`self.Couleur`)))
  ;[1 1 1] Lance un event toutes les frames
  (`LightComponent.SetLightColor` (`self.PointLight`) (make `LinearColor` _couleur_x _couleur_y _couleur_z 1.0) true))

(event `Key|Multiply`
  (params (Key :type "Key Structure"))
  ;[1 1 1] Changement de couleur
  (:`Pressed`
    (set `self.Couleur` (`KismetMathLibrary.MakeVector` (+ (.x (`self.Couleur`)) 1.0) (.y (`self.Couleur`)) (.z (`self.Couleur`))))))

(event `self.ReceiveBeginPlay`
  ;[1 1 1] Active la prise en compte du clic
  (`self.EnableInput` (`GameplayStatics.GetPlayerController` 0)))

(event `Key|Divide`
  (params (Key :type "Key Structure"))
  ;[1 1 1] Changement de couleur
  (:`Pressed`
    (set `self.Couleur` (`KismetMathLibrary.MakeVector` (- (.x (`self.Couleur`)) 1.0) (.y (`self.Couleur`)) (.z (`self.Couleur`))))))

(fn `UserConstructionScript`)