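; FunctionActor is an actor that finds a tagged lamp and prints a message describing its point light intensity every frame.
; Tick searches by tag, casts the first result to Lampe_BP_intensity, stores it and prints an error if the cast or validity check fails.
; GetLightIntensity compares the intensity to a threshold, returning a "large" message or delegating to Réponse 1, whose "small" message node appears unconnected.
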(event `self.ReceiveTick`
  (params (DeltaSeconds :type "Float (single-precision)"))
  ;[1 1 1] GET Lampe BP,  je la met dans une variable, on check qu'elle existe bien, puis on appelle la fonction
  (bind _outactors (`GameplayStatics.GetAllActorsWithTag` "LampeBPI ntensity"))
  (bind _aslampe_bp_intensity (cast `/Game/Blueprints/Lampe_BP_intensity` (`|GetArrayItem` _outactors))
    (:`then`
      (bind _output_get (set `self.Lampe` _aslampe_bp_intensity))
      (`/Engine/EditorBlueprintResources/StandardMacros.IsValid` _output_get
        (:`Is Valid`
          (bind `_réponse` (`self.GetLightIntensity` (`/Game/Blueprints/Lampe_BP_intensity.PointLight` (`self.Lampe`))))
          (`KismetSystemLibrary.PrintString` `_réponse` true true (struct :`G` 0.147163 :`B` 1.0 :`A` 1.0)))
        (:`Is Not Valid`
          (`KismetSystemLibrary.PrintString` "Lampe non trouvée" true true (struct :`R` 1.0 :`B` 0.006282 :`A` 1.0)))))
    (:`CastFailed`
      (`KismetSystemLibrary.PrintString` "Pas le bon type pour le tag" true true (struct :`R` 1.0 :`B` 0.029008 :`A` 1.0)))))

(fn `GetLightIntensity`
  (params (Light :type "PointLightComponent Object Reference"))
  (returns (`Réponse` :type String))
  (bind _output_get (set `self.Intensity` (`LightComponentBase.Intensity` Light)))
  (if (< _output_get 500.0)
    (return (`self.Réponse 1`))
    (else
      (return (`KismetStringLibrary.Concat_StrStr` "L'intensité est grande : " (`KismetStringLibrary.Conv_DoubleToString` (`self.Intensity`)))))))

(fn `UserConstructionScript`)