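; Lamp Blueprint that lets the player raise or lower the brightness of its point light with the keyboard.
; BeginPlay enables input from player controller 0, and the Add and Subtract keys step an intensity variable up or down by a fixed amount.
; Tick applies that variable to the PointLight intensity every frame, with no clamping on the value.
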(event `self.ReceiveTick`
  (params (DeltaSeconds :type "Float (single-precision)"))
  ;[1 1 1] Lance un event toutes les frames
  (`LightComponent.SetIntensity` (`self.PointLight`) (`KismetMathLibrary.Conv_IntToDouble` (`self.Intensité`))))

(event `Key|Add`
  (params (Key :type "Key Structure"))
  ;[1 1 1] Modifie l'intensité en appuyant sur + ou -
  (:`Pressed`
    (set `self.Intensité` (+ (`self.Intensité`) 200))))

(event `Key|Subtract`
  (params (Key :type "Key Structure"))
  ;[1 1 1] Modifie l'intensité en appuyant sur + ou -
  (:`Pressed`
    (set `self.Intensité` (- (`self.Intensité`) 200))))

(event `self.ReceiveBeginPlay`
  ;[1 1 1] Active la prise en compte du clic
  (`self.EnableInput` (`GameplayStatics.GetPlayerController` 0)))

(fn `UserConstructionScript`)