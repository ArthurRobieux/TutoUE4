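; Collectible coin that spins and bobs in place, and is picked up when the hero overlaps its box.
; Tick rotates the mesh, while a timeline offsets its height from the Z saved at BeginPlay, alternating forward and reverse through a FlipFlop re-triggered on finish.
; On overlap with Hero_BP, it plays a sound, increments the hero's Coin counter and destroys itself.
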(event `self.ReceiveBeginPlay`
  (bind (_returnvalue_x _returnvalue_y _returnvalue_z) (`KismetMathLibrary.BreakVector` (`SceneComponent.K2_GetComponentLocation` (`self.StaticMesh`))))
  ;[1 1 1] Initialisation
  (set `self.PositionZInitiale` _returnvalue_z)
  (`self.UpDown`))

(event `self.ReceiveTick`
  (params (DeltaSeconds :type "Float (single-precision)"))
  ;[1 1 1] Rotation
  (`SceneComponent.K2_AddRelativeRotation` (`self.StaticMesh`) (struct :`Yaw` 2.0) false false))

(event `UpDown`
  (bind _staticmesh (`self.StaticMesh`))
  (bind (_returnvalue_x _returnvalue_y) (`KismetMathLibrary.BreakVector` (`SceneComponent.K2_GetComponentLocation` _staticmesh)))
  ;[1 1 1] Up / Down
  (`/Engine/EditorBlueprintResources/StandardMacros.FlipFlop`
    (:`A`
      (bind (_direction _newtrack_0) (`Timeline|Timeline_0` :!via `PlayFromStart` :!label _label)
        (:`Update`
          (`SceneComponent.K2_SetWorldLocation` _staticmesh (`KismetMathLibrary.MakeVector` _returnvalue_x _returnvalue_y (+ (* _newtrack_0 10.0) (`self.PositionZInitiale`))) false false))
        (:`Finished`
          (`self.UpDown`))))
    (:`B`
      (goto _label :!via `ReverseFromEnd`))))

(event `self.Box.OnComponentBeginOverlap`
  (params (OverlappedComponent :type "PrimitiveComponent Object Reference") (OtherActor :type "Actor Object Reference") (OtherComp :type "PrimitiveComponent Object Reference") (OtherBodyIndex :type Integer) (bFromSweep :type Boolean) (SweepResult :type "HitResult Structure (by ref)"))
  ;[1 1 1] Collect coin
  (bind _ashero_bp (cast `/Game/Hero/Hero_BP` OtherActor))
  (`GameplayStatics.SpawnSoundAtLocation` "/Game/Coin/CoinSoundEffect.CoinSoundEffect" (`self.K2_GetActorLocation`) (struct) 0.5 1.0 0.0 null null)
  (`/Engine/EditorBlueprintResources/StandardMacros.IncrementInt` (`/Game/Hero/Hero_BP.Coin` _ashero_bp)
    (:`  `
      (`self.K2_DestroyActor`))))

(fn `UserConstructionScript`)